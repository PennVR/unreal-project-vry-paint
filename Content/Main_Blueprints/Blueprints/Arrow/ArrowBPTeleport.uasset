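; Teleport arrow projectile that moves the player to where it lands.
; On hit, it teleports player 0 to the impact point if the struck actor is tagged "teleportable", then destroys itself either way.
; It also clears the FirstPersonCharacter's TeleportArrowPresent flag.
; The construction script sets the projectile's initial speed from an InitSpeed variable.
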(event `self.ReceiveHit`
  (params (MyComp :type "PrimitiveComponent Object Reference") (Other :type "Actor Object Reference") (OtherComp :type "PrimitiveComponent Object Reference") (bSelfMoved :type Boolean) (HitLocation :type "Vector Structure") (HitNormal :type "Vector Structure") (NormalImpulse :type "Vector Structure") (Hit :type "HitResult Structure (by ref)"))
  (bind _returnvalue (`GameplayStatics.GetPlayerCharacter` 0))
  ;[1 1 1] Teleport the main character if we hit a teleportable surface
  (if (`KismetArrayLibrary.Array_Contains` (`Actor.Tags` Other) "teleportable")
    (`self.K2_SetActorLocation` _returnvalue HitLocation false false))
  (`self.K2_DestroyActor`) ; Then destroy this projectile
  (bind _asfirst_person_character (cast `/Game/Main_Blueprints/Blueprints/Bow/FirstPersonCharacter` _returnvalue))
  (set `/Game/Main_Blueprints/Blueprints/Bow/FirstPersonCharacter.TeleportArrowPresent` false _asfirst_person_character))

(fn `UserConstructionScript`
  (set `ProjectileMovementComponent.InitialSpeed` (`self.InitSpeed`) (`self.Projectile`)))